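; BP_Cube is a debug-style actor in MatchCircuit that is nudged along the world X axis from the keyboard.
; BeginPlay enables input from player controller 0, so debug keys U and J teleport-step it forward and back by a fixed offset, without sweep.
; Tick prints its current location on screen every frame under a single key.
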(event EventBeginPlay
  (Input|EnableInput (Game|GetPlayerController 0)))

(event Collision|EventActorBeginOverlap
  (params (OtherActor :type Actor%20Object%20Reference)))

(event EventTick
  (params (DeltaSeconds :type Float%20%28single-precision%29))
  (Development|PrintString (Utilities|String|ToString(Vector) (Transformation|GetActorLocation)) true true "(R=0.000000,G=0.660000,B=1.000000,A=1.000000)" 2.0 "1"))

(event Input|KeyboardEvents|DebugKeyU
  (params (Key :type Key%20Structure :default "None") (ActionValue :type Input%20Action%20Value%20Structure))
  (bind _returnvalue (Transformation|GetActorLocation))
  (bind (_x _y _z) (Math|Vector|BreakVector _returnvalue))
  (:Pressed
    (Transformation|SetActorLocation (Math|Vector|MakeVector (+ _x 2e+01) _y _z) false false)))

(event Input|KeyboardEvents|DebugKeyJ
  (params (Key :type Key%20Structure :default "None") (ActionValue :type Input%20Action%20Value%20Structure))
  (bind _returnvalue (Transformation|GetActorLocation))
  (bind (_x _y _z) (Math|Vector|BreakVector _returnvalue))
  (:Pressed
    (Transformation|SetActorLocation (Math|Vector|MakeVector (+ _x -2e+01) _y _z) false false)))

(fn ConstructionScript)