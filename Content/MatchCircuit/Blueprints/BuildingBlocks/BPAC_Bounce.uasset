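; Actor component for a laser circuit that bounces incoming lasers off its owner, like a mirror.
; Each new hit spawns a BPSC_Emitter on the owner at the reflected location and rotation, tracked in a map keyed by the incoming laser.
; Hit updates move that emitter, and hit end stops and destroys it.
; IntermediateChange refreshes the color of all bounced lasers.
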(event `self.ReceiveBeginPlay`
  (bind _returnvalue (`Actor.GetComponentByClass` (`self.GetOwner`) "/Game/MatchCircuit/Blueprints/BuildingBlocks/BPAC_Handler.BPAC_Handler_C"))
  (`/Engine/EditorBlueprintResources/StandardMacros.IsValid` _returnvalue
    (:`Is Valid`
      (set `self.OwningHandler` _returnvalue))))

(event `/Game/MatchCircuit/Blueprints/BuildingBlocks/BPI_Lasers.LaserStartHitting`
  (params (Input :type "/Game/MatchCircuit/Blueprints/BuildingBlocks/BP_Laser Object Reference") (HitInfo :type "HitResult Structure"))
  (`/Engine/EditorBlueprintResources/StandardMacros.IsValid` Input
    (:`Is Valid`
      (`self.MapContainsLaser` Input
        (:`False`
          (`self.SpawnLaser` Input HitInfo))))))

(event `/Game/MatchCircuit/Blueprints/BuildingBlocks/BPI_Lasers.LaserStopHitting`
  (params (Input :type "/Game/MatchCircuit/Blueprints/BuildingBlocks/BP_Laser Object Reference"))
  (`self.RemoveLaser` Input))

(event `/Game/MatchCircuit/Blueprints/BuildingBlocks/BPI_Lasers.LaserUpdateHitting`
  (params (Input :type "/Game/MatchCircuit/Blueprints/BuildingBlocks/BP_Laser Object Reference") (HitInfo :type "HitResult Structure"))
  (bind (_outputpin _returnvalue) (`self.MirrorLocationRotation` HitInfo))
  (bind _emitter (`self.FindLaserOnMap` Input)
    (:`then`
      (`SceneComponent.K2_SetWorldLocationAndRotation` _emitter _outputpin _returnvalue false false))))

(event `/Game/MatchCircuit/Blueprints/BuildingBlocks/BPI_Lasers.IntermediateChange`
  (params (Modified :type "/Game/MatchCircuit/Blueprints/BuildingBlocks/BP_Laser Object Reference"))
  (bind _values (`BlueprintMapLibrary.Map_Values` (`self.EmitterBounceMap`)))
  (for _array_element _values
    (`/Game/MatchCircuit/Blueprints/BuildingBlocks/BPSC_Emitter.SetLaserColor` _array_element)))

(fn `RemoveLaser`
  (params (InputPin :type "/Game/MatchCircuit/Blueprints/BuildingBlocks/BP_Laser Object Reference"))
  (locals (ItemToRemove :type "/Game/MatchCircuit/Blueprints/BuildingBlocks/BPSC_Emitter Object Reference"))
  (bind _emitter (`self.FindLaserOnMap` (`local.InputPin`))
    (:`then`
      (bind _output_get (set `local.ItemToRemove` _emitter))
      (`/Game/MatchCircuit/Blueprints/BuildingBlocks/BPSC_Emitter.LaserStopHitting` _output_get null)
      (`self.K2_DestroyComponent` (`local.ItemToRemove`))
      (`BlueprintMapLibrary.Map_Remove` (`self.EmitterBounceMap`) (`local.InputPin`)))))

(fn `SpawnLaser`
  (params (LaserIn :type "/Game/MatchCircuit/Blueprints/BuildingBlocks/BP_Laser Object Reference") (hitInfo :type "HitResult Structure"))
  (bind _returnvalue (`Actor.GetTransform` (`self.GetOwner`)))
  (bind (_outputpin _returnvalue_2) (`self.MirrorLocationRotation` (`local.hitInfo`)))
  (bind _returnvalue_3 (`|AddComponentByClass` (`self.GetOwner`) "/Game/MatchCircuit/Blueprints/BuildingBlocks/BPSC_Emitter.BPSC_Emitter_C" false (`KismetMathLibrary.MakeTransform` (`KismetMathLibrary.InverseTransformLocation` _returnvalue _outputpin) (`KismetMathLibrary.InverseTransformRotation` _returnvalue _returnvalue_2))))
  (`BlueprintMapLibrary.Map_Add` (`self.EmitterBounceMap`) (`local.LaserIn`) _returnvalue_3)
  (`/Game/MatchCircuit/Blueprints/BuildingBlocks/BPSC_Emitter.SetLaserColor` _returnvalue_3)
  (`/Game/MatchCircuit/Blueprints/BuildingBlocks/BPSC_Emitter.ActivateLaser` _returnvalue_3))