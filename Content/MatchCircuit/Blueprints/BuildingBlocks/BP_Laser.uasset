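; Laser beam building block that traces forward each tick, scales its mesh to the blocking hit and notifies hit actors' BPAC_Handler components.
; It diffs current and previous handler sets to send start and stop messages only on change.
; A recursive check through upstream lasers' owning handlers filters hits to guard against loops.
; When told to stop, it notifies previously hit handlers, then destroys itself.
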(event `self.ReceiveBeginPlay`
  (bind _returnvalue (`PrimitiveComponent.CreateDynamicMaterialInstance` (`self.StaticMesh`) 0 "/Game/MatchCircuit/Assets/Materials/MI_Laser.MI_Laser" "None"))
  (set `self.LaserMaterial` _returnvalue)
  (`self.SetLaserColor` (`self.ColorOverride`)))

(event `self.ReceiveTick`
  (params (DeltaSeconds :type "Float (single-precision)"))
  (bind _returnvalue (`self.K2_GetActorLocation`))
  (`self.UpdateLength` (`self.Range`))
  (bind _outhits (`KismetSystemLibrary.SphereTraceMulti` _returnvalue (+ _returnvalue (* (`self.GetActorForwardVector`) (`self.Range`))) 0.5 "TraceTypeQuery3" false (`self.ActorsToIgnore`)))
  (for _array_element _outhits
    (`|ExecutionSequence`
      (:`then_0`
        (bind (_bblockinghit _binitialoverlap _time _distance) (`GameplayStatics.BreakHitResult` _array_element))
        (if _bblockinghit
          (`self.UpdateLength` _distance)))
      (:`then_1`
        (`self.HandleHitActors` _array_element))))
  (bind _result (`BlueprintSetLibrary.Set_Difference` (`self.PreviouslyHitHandlers`) (`self.CurrentHitHandlers`)))
  (bind _result_2 (`BlueprintSetLibrary.Set_ToArray` _result))
  (for _array_element_2 _result_2
    (message `/Game/MatchCircuit/Blueprints/BuildingBlocks/BPI_Lasers.LaserStopHitting` _array_element_2 self)
    (`BlueprintMapLibrary.Map_Remove` (`self.HittingHandlers`) _array_element_2))
  (set `self.PreviouslyHitHandlers` (`self.CurrentHitHandlers`))
  (`BlueprintSetLibrary.Set_Clear` (`self.CurrentHitHandlers`)))

(event `/Game/MatchCircuit/Blueprints/BuildingBlocks/BPI_Lasers.LaserStopHitting`
  (params (Input :type "/Game/MatchCircuit/Blueprints/BuildingBlocks/BP_Laser Object Reference"))
  (`|ExecutionSequence`
    (:`then_0`
      (bind _result (`BlueprintSetLibrary.Set_ToArray` (`self.PreviouslyHitHandlers`)))
      (for _array_element _result
        (message `/Game/MatchCircuit/Blueprints/BuildingBlocks/BPI_Lasers.LaserStopHitting` _array_element self)))
    (:`then_1`
      (`self.K2_DestroyActor`))))

(fn `DebugSet`
  (params (Set :type "Set of /Game/MatchCircuit/Blueprints/BuildingBlocks/BPAC_Handler Object Reference (by ref)") (Prefix :type String))
  (bind _result (`BlueprintSetLibrary.Set_ToArray` Set))
  (for _array_element _result
    (bind _returnvalue (`KismetStringLibrary.Concat_StrStr` Prefix (`KismetSystemLibrary.GetDisplayName` _array_element)))
    (`KismetSystemLibrary.PrintString` _returnvalue true true (struct :`G` 0.66 :`B` 1.0 :`A` 1.0) (`GameplayStatics.GetWorldDeltaSeconds`) (`KismetStringLibrary.Conv_StringToName` _returnvalue))))

(fn `HandleHitActors`
  (params (InputPin :type "HitResult Structure"))
  (locals (HandlerLocal :type "/Game/MatchCircuit/Blueprints/BuildingBlocks/BPAC_Handler Object Reference"))
  (bind _returnvalue (`self.GetComponentByClass` (`.HitActor` (`GameplayStatics.BreakHitResult` (`local.InputPin`))) "/Game/MatchCircuit/Blueprints/BuildingBlocks/BPAC_Handler.BPAC_Handler_C"))
  (`/Engine/EditorBlueprintResources/StandardMacros.IsValid` _returnvalue
    (:`Is Valid`
      (set `local.HandlerLocal` _returnvalue)
      (if (`self.IsNotOnPath` (`local.HandlerLocal`))
        (`BlueprintMapLibrary.Map_Add` (`self.HittingHandlers`) (`local.HandlerLocal`) (`local.InputPin`))
        (if (not (`BlueprintSetLibrary.Set_Contains` (`self.PreviouslyHitHandlers`) (`local.HandlerLocal`)))
          (message `/Game/MatchCircuit/Blueprints/BuildingBlocks/BPI_Lasers.LaserStartHitting` (`local.HandlerLocal`) self (`local.InputPin`)))
        (`BlueprintSetLibrary.Set_Add` (`self.CurrentHitHandlers`) (`local.HandlerLocal`))))))

(fn `IsNotOnPath`
  (params (InputHandler :type "/Game/MatchCircuit/Blueprints/BuildingBlocks/BPAC_Handler Object Reference"))
  (returns (OutputPin :type Boolean))
  (locals (CurrentLaser :type "/Game/MatchCircuit/Blueprints/BuildingBlocks/BP_Laser Object Reference"))
  (if (`KismetArrayLibrary.Array_IsNotEmpty` (`self.PreviousLasers`))
    (for _array_element (`self.PreviousLasers`)
      (bind _output_get (set `local.CurrentLaser` _array_element))
      (if (== (`/Game/MatchCircuit/Blueprints/BuildingBlocks/BP_Laser.OwningHandler` _output_get) (`self.OwningHandler`))
        (return false)
        (elif (not (`self.IsNotOnPath` (`local.CurrentLaser`) (`local.InputHandler`)))
          (return false))))
    (return true)
    (else
      (return true))))

(fn `SetLaserColor`
  (params (Value :type "LinearColor Structure"))
  (`MaterialInstanceDynamic.SetVectorParameterValue` (`self.LaserMaterial`) "BaseColor" Value))

(fn `UpdateLength`
  (params (InputPin :type "Float (single-precision)"))
  (if (not (`KismetMathLibrary.NearlyEqual_FloatFloat` InputPin (`self.PreviousLength`)))
    (bind _output_get (set `self.PreviousLength` (`local.InputPin`)))
    (`SceneComponent.SetWorldScale3D` (`self.StaticMesh`) (`KismetMathLibrary.MakeVector` 0.1 0.1 (/ _output_get 100.0)))))

(fn `UserConstructionScript`)