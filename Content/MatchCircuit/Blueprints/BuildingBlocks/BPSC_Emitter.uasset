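; BPSC_Emitter is a scene component building block for MatchCircuit that emits a laser when activated.
; On BeginPlay it caches the owner's BPAC_Handler; laser hit start and stop events activate or deactivate emission, swapped when the system is inverted.
; Activation spawns an attached BP_Laser with color, range, previous lasers and handler, ignoring the owner.
; Deactivation forwards LaserStopHitting to that laser.
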(event `self.ReceiveBeginPlay`
  (bind _returnvalue (`Actor.GetComponentByClass` (`self.GetOwner`) "/Game/MatchCircuit/Blueprints/BuildingBlocks/BPAC_Handler.BPAC_Handler_C"))
  (`/Engine/EditorBlueprintResources/StandardMacros.IsValid` _returnvalue
    (:`Is Valid`
      (set `self.OwningHandler` _returnvalue))))

(event `/Game/MatchCircuit/Blueprints/BuildingBlocks/BPI_Lasers.LaserStartHitting`
  (params (Input :type "/Game/MatchCircuit/Blueprints/BuildingBlocks/BP_Laser Object Reference") (HitInfo :type "HitResult Structure"))
  (if (`self.IsSystemInverted`)
    (`self.DeactivateLaser`)
    (else
      (`self.ActivateLaser`))))

(event `/Game/MatchCircuit/Blueprints/BuildingBlocks/BPI_Lasers.LaserStopHitting`
  (params (Input :type "/Game/MatchCircuit/Blueprints/BuildingBlocks/BP_Laser Object Reference"))
  (if (`self.IsSystemInverted`)
    (`self.ActivateLaser`)
    (else
      (`self.DeactivateLaser`))))

(fn `ActivateLaser`
  (bind _returnvalue (`|SpawnActorFromClass` "/Game/MatchCircuit/Blueprints/BuildingBlocks/BP_Laser.BP_Laser_C" (`self.K2_GetComponentToWorld`) "Undefined" "MultiplyWithRoot" null (`self.CurrentColor`) (`self.MaxRange`) (`self.GetFilteredLasers`) (`self.OwningHandler`) (`|MakeArray` (`self.GetOwner`)) null))
  (bind _output_get (set `self.AttachedLaser` _returnvalue))
  (`Actor.K2_AttachToComponent` _output_get self "None" "KeepWorld" "KeepWorld" "KeepWorld" false))

(fn `DeactivateLaser`
  (bind _attachedlaser (`self.AttachedLaser`)
    (:`then`
      (`/Game/MatchCircuit/Blueprints/BuildingBlocks/BP_Laser.LaserStopHitting` _attachedlaser null))
    (:`else`
      (`KismetSystemLibrary.PrintString` "Attached Laser is not valid from Emitter" true true (struct :`R` 1.0 :`A` 1.0)))))