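; Actor component that acts as the laser hub for its owner, relaying hit events to the owner's other BPI_Lasers components.
; On BeginPlay it caches those components, sets mesh laser-channel collision to block or overlap, and stops hits on emitters if InvertSystem is set.
; Start and stop events update the laser queue and forward only when unlocked, while update events always forward.
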(event `self.ReceiveBeginPlay`
  (`|ExecutionSequence`
    (:`then_0`
      (set `self.LinkedComponents` (`Actor.GetComponentsByInterface` (`self.GetOwner`) "/Game/MatchCircuit/Blueprints/BuildingBlocks/BPI_Lasers.BPI_Lasers_C"))
      (`KismetArrayLibrary.Array_RemoveItem` (`self.LinkedComponents`) self)
      (for _array_element (`Actor.K2_GetComponentsByClass` (`self.GetOwner`) "/Script/Engine.StaticMeshComponent")
        (`PrimitiveComponent.SetCollisionResponseToChannel` _array_element "ECC_GameTraceChannel1" (select `bool` (`self.bIsBlocking`) :`false` "ECR_Overlap" :`true` "ECR_Block" :!type "ECollisionResponse Enum"))))
    (:`then_1`
      (if (`self.bInvertSystem`)
        (for _array_element_2 (`Actor.K2_GetComponentsByClass` (`self.GetOwner`) "/Game/MatchCircuit/Blueprints/BuildingBlocks/BPSC_Emitter.BPSC_Emitter_C")
          (`/Game/MatchCircuit/Blueprints/BuildingBlocks/BPSC_Emitter.LaserStopHitting` _array_element_2 null))))))

(event `/Game/MatchCircuit/Blueprints/BuildingBlocks/BPI_Lasers.LaserStartHitting`
  (params (Input :type "/Game/MatchCircuit/Blueprints/BuildingBlocks/BP_Laser Object Reference") (HitInfo :type "HitResult Structure"))
  (`self.LaserAdded` Input)
  (`self.IsNotLocked`
    (:`Not Locked`
      (bind _array_element (`self.ForEachComponent`)
        (:`LoopBody`
          (message `/Game/MatchCircuit/Blueprints/BuildingBlocks/BPI_Lasers.LaserStartHitting` _array_element Input HitInfo))))))

(event `/Game/MatchCircuit/Blueprints/BuildingBlocks/BPI_Lasers.LaserStopHitting`
  (params (Input :type "/Game/MatchCircuit/Blueprints/BuildingBlocks/BP_Laser Object Reference"))
  (`self.LaserRemoved` Input)
  (`self.IsNotLocked`
    (:`Not Locked`
      (bind _array_element (`self.ForEachComponent`)
        (:`LoopBody`
          (message `/Game/MatchCircuit/Blueprints/BuildingBlocks/BPI_Lasers.LaserStopHitting` _array_element Input))))))

(event `/Game/MatchCircuit/Blueprints/BuildingBlocks/BPI_Lasers.LaserUpdateHitting`
  (params (Input :type "/Game/MatchCircuit/Blueprints/BuildingBlocks/BP_Laser Object Reference") (HitInfo :type "HitResult Structure"))
  (bind _array_element (`self.ForEachComponent`)
    (:`LoopBody`
      (message `/Game/MatchCircuit/Blueprints/BuildingBlocks/BPI_Lasers.LaserUpdateHitting` _array_element Input HitInfo))))

(fn `LaserAdded`
  (params (NewLaser :type "/Game/MatchCircuit/Blueprints/BuildingBlocks/BP_Laser Object Reference (by ref)"))
  (`KismetArrayLibrary.Array_AddUnique` (`self.LasersInQueue`) NewLaser))

(fn `LaserRemoved`
  (params (LaserToRemove :type "/Game/MatchCircuit/Blueprints/BuildingBlocks/BP_Laser Object Reference (by ref)"))
  (`KismetArrayLibrary.Array_RemoveItem` (`self.LasersInQueue`) LaserToRemove))